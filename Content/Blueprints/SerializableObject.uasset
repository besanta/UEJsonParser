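; SerializableObject captures a snapshot of a pawn and converts it to and from a JSON data object.
; Construct records control state, name, speed, class, the current time and the controller's transform, both whole and split.
; Serialize writes these under string keys, nesting location, rotation and scale and packing date parts, year included, into single bytes.
; Unserialize restores the variables from valid data and returns itself, without applying them to any actor.
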(fn `Construct`
  (params (Target :type "Pawn Object Reference"))
  (bind _returnvalue (`Actor.GetTransform` (`Pawn.GetController` Target)))
  (`|ExecutionSequence`
    (:`then_0`
      (set `self.IsControlled` (`Pawn.IsPlayerControlled` Target))
      (set `self.Name` (`KismetSystemLibrary.GetObjectName` Target)))
    (:`then_1`
      (set `self.Transform` _returnvalue)
      (set `self.Location` (.location _returnvalue))
      (set `self.Rotation` (.rotation _returnvalue))
      (set `self.Scale` (.scale _returnvalue)))
    (:`then_2`
      (set `self.Class` (`GameplayStatics.GetObjectClass` Target)))
    (:`then_3`
      (set `self.DateTime` (`KismetMathLibrary.Now`)))
    (:`then_4`
      (set `self.Velocity` (`KismetMathLibrary.VSize` (`Actor.GetVelocity` Target))))))

(fn `Serialize`
  (returns (JSONData :type "JsonFieldData Object Reference"))
  (locals (JSONDataObject :type "JsonFieldData Object Reference"))
  (bind (_year _month _day _hour _minute _second _millisecond) (`KismetMathLibrary.BreakDateTime` (`self.DateTime`)))
  (`|ExecutionSequence`
    (:`then_0`
      (set `local.JSONDataObject` (`JsonFieldData.Create`)))
    (:`then_1`
      (set `local.JSONDataObject` (`JsonFieldData.SetNumber` (`JsonFieldData.SetString` (`JsonFieldData.SetBool` (`local.JSONDataObject`) "Is Player Controlled" (`self.IsControlled`)) "Player Name" (`self.Name`)) "Velocity" (`self.Velocity`))))
    (:`then_2`
      (set `local.JSONDataObject` (`JsonFieldData.SetObject` (`JsonFieldData.SetTranform` (`local.JSONDataObject`) "Transform" (`self.Transform`)) "Break Transform" (`JsonFieldData.SetVector` (`JsonFieldData.SetRotator` (`JsonFieldData.SetVector` (`JsonFieldData.Create`) "Location" (`self.Location`)) "Rotation" (`self.Rotation`)) "Scale" (`self.Scale`)))))
    (:`then_3`
      (set `local.JSONDataObject` (`JsonFieldData.SetClass` (`local.JSONDataObject`) "Class" (`self.Class`))))
    (:`then_4`
      (set `local.JSONDataObject` (`JsonFieldData.SetByteArray` (`local.JSONDataObject`) "DateTime" (`|MakeArray` (`KismetMathLibrary.Conv_IntToByte` _year) (`KismetMathLibrary.Conv_IntToByte` _month) (`KismetMathLibrary.Conv_IntToByte` _day) (`KismetMathLibrary.Conv_IntToByte` _hour) (`KismetMathLibrary.Conv_IntToByte` _minute) (`KismetMathLibrary.Conv_IntToByte` _second) (`KismetMathLibrary.Conv_IntToByte` _millisecond)))))
    (:`then_5`
      (return (`local.JSONDataObject`)))))

(fn `Unserialize`
  (params (JSONData :type "JsonFieldData Object Reference"))
  (returns (Object :type "/Game/Blueprints/SerializableObject Object Reference"))
  (bind _returnvalue (`JsonFieldData.GetObject` JSONData "Break Transform"))
  (bind _returnvalue_2 (`JsonFieldData.GetByteArray` JSONData "DateTime"))
  (`/Engine/EditorBlueprintResources/StandardMacros.IsValid` JSONData
    (:`Is Valid`
      (`|ExecutionSequence`
        (:`then_0`
          (set `self.IsControlled` (`JsonFieldData.GetBool` JSONData "Is Player Controlled"))
          (set `self.Name` (`JsonFieldData.GetString` JSONData "Player Name"))
          (set `self.Velocity` (`JsonFieldData.GetNumber` JSONData "Velocity")))
        (:`then_1`
          (set `self.Transform` (`JsonFieldData.GetTransform` JSONData "Transform"))
          (set `self.Location` (`JsonFieldData.GetVector` _returnvalue "Location"))
          (set `self.Rotation` (`JsonFieldData.GetRotator` _returnvalue "Rotation"))
          (set `self.Scale` (`JsonFieldData.GetVector` _returnvalue "Scale")))
        (:`then_2`
          (set `self.Class` (`JsonFieldData.GetClass` JSONData "Class")))
        (:`then_3`
          (set `self.DateTime` (`KismetMathLibrary.MakeDateTime` (`KismetMathLibrary.Conv_ByteToInt` (`|GetArrayItem` _returnvalue_2)) (`KismetMathLibrary.Conv_ByteToInt` (`|GetArrayItem` _returnvalue_2 1)) (`KismetMathLibrary.Conv_ByteToInt` (`|GetArrayItem` _returnvalue_2 2)) (`KismetMathLibrary.Conv_ByteToInt` (`|GetArrayItem` _returnvalue_2 3)) (`KismetMathLibrary.Conv_ByteToInt` (`|GetArrayItem` _returnvalue_2 4)) (`KismetMathLibrary.Conv_ByteToInt` (`|GetArrayItem` _returnvalue_2 5)) (`KismetMathLibrary.Conv_ByteToInt` (`|GetArrayItem` _returnvalue_2 6)))))
        (:`then_4`
          (return self))))
    (:`Is Not Valid`
      (return self))))