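; Writer is an actor Blueprint that periodically serializes the player pawn into a shared Data archive.
; Tick runs through a one-second Delay, then constructs a new SerializableObject from player 0's pawn.
; It prints the serialized content string for debugging and, if Data is valid, serializes again to update that archive.
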(event `self.ReceiveTick`
  (params (DeltaSeconds :type "Float (single-precision)"))
  (bind _data (`self.Data`))
  (`KismetSystemLibrary.Delay` 1.0)
  (bind _returnvalue (`|GenericCreateObject` "/Game/Blueprints/SerializableObject.SerializableObject_C" self))
  (`/Game/Blueprints/SerializableObject.Construct` _returnvalue (`GameplayStatics.GetPlayerPawn` 0))
  (bind _jsondata (`/Game/Blueprints/SerializableObject.Serialize` _returnvalue))
  (`KismetSystemLibrary.PrintString` (`JsonFieldData.GetContentString` _jsondata) true true (struct :`R` 1.0 :`G` 0.046851 :`A` 1.0))
  (`/Engine/EditorBlueprintResources/StandardMacros.IsValid` _data
    (:`Is Valid`
      (`/Game/Blueprints/DataActor.UpdateArchive` _data _jsondata))))

(fn `UserConstructionScript`)