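; Automated test Blueprint for a JSON object library, checking round trips of each supported value type.
; UnitTest runs each case: values are set on a JSON object, serialized to a string, parsed back and compared, with pass/fail stored in a Tests map.
; Coverage includes arrays, UObjects, structs, containers, engine math types, a base64 texture, and async HTTP and file loads.
; DisplayResults runs after a short delay.
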(event `self.ReceiveBeginPlay`)

(event `UnitTest`
  (`|ExecutionSequence`
    (:`then_0`
      ;[1 1 1] Test Sequence
      (`|ExecutionSequence`
        (:`then_0`
          (`self.Test_01_Add_Boolean`)
          (`self.Test_06_Add_Array_Boolean`))
        (:`then_1`
          (`self.Test_02_Add_String`)
          (`self.Test_07_Add_Array_String`))
        (:`then_2`
          (`self.Test_03_Add_Number`)
          (`self.Test_08_Add_Array_Number`))
        (:`then_3`
          (`self.Test_04_Add_Object`)
          (`self.Test_05_Add_Null`))
        (:`then_4`
          (`self.Test_16_Add_Color`)
          (`self.Test_16_Add_Vector`)
          (`self.Test_16_Add_Rotator`)
          (`self.Test16_Add_Transform`)
          (`self.Test_16_Add_Name`))
        (:`then_5`
          (`self.Test_11_Add_UObject`))
        (:`then_6`
          (`self.Test_11_Add_UStruct`)
          (`self.Test_11_Add_UStruct_Array`)
          (`self.Test_11_Add_Map`)
          (`self.Test_11_Add_Set`))
        (:`then_7`
          (`self.Test_Async_From_HTTP`)
          (`self.Test_Async From_File`))
        (:`then_8`
          (`self.Test_17_Load_Texture`)
          (`self.Test_17_Copy_JSON`))))
    (:`then_1`
      (`KismetSystemLibrary.Delay` 2.0)
      (bind _keys (`BlueprintMapLibrary.Map_Keys` (`self.Tests`)))
      (for _array_element _keys
        (`KismetSystemLibrary.PrintText` (`|FormatText` "TEST {A} : {STATE}" _array_element (`KismetMathLibrary.SelectString` "SUCCESS" "FAILLURE" (`BlueprintMapLibrary.Map_Find` (`self.Tests`) _array_element))) false)))))

(event `Test_01_Add_Boolean`
  (bind _returnvalue (`JsonFieldData.CreateFromString` (`JsonFieldData.GetContentString` (`JsonFieldData.SetBool` (`JsonFieldData.SetBool` (`JsonFieldData.Create`) "booltrue" true) "boolfalse" false))))
  ;[1 1 1] JSON Types
  (`BlueprintMapLibrary.Map_Add` (`self.Tests`) "Test_01_Add_Boolean" (!= (`JsonFieldData.GetBool` _returnvalue "booltrue") (`JsonFieldData.GetBool` _returnvalue "boolfalse"))))

(event `Test_06_Add_Array_Boolean`
  (bind _array (`|MakeArray` false true))
  (bind _returnvalue (`JsonFieldData.GetBoolArray` (`JsonFieldData.CreateFromString` (`JsonFieldData.GetContentString` (`JsonFieldData.SetAnyProperty` (`JsonFieldData.SetBoolArray` (`JsonFieldData.Create`) "booleans" _array) "ANYbool" _array))) "booleans"))
  ;[1 1 1] Arrays of JSON Types
  (`BlueprintMapLibrary.Map_Add` (`self.Tests`) "Test_13_Add_Boolean_Array" (!= (`|GetArrayItem` _returnvalue) (`|GetArrayItem` _returnvalue 1))))

(event `Test_02_Add_String`
  (bind _dummystring (`self.DummyString`))
  ;[1 1 1] JSON Types
  (`BlueprintMapLibrary.Map_Add` (`self.Tests`) "Test_02_Add_String" (`KismetStringLibrary.EqualEqual_StrStr` (`JsonFieldData.GetString` (`JsonFieldData.CreateFromString` (`JsonFieldData.GetContentString` (`JsonFieldData.SetString` (`JsonFieldData.Create`) "string" _dummystring))) "string") _dummystring)))

(event `Test_07_Add_Array_String`
  ;[1 1 1] Arrays of JSON Types
  (`BlueprintMapLibrary.Map_Add` (`self.Tests`) "Test_13_Add_String_Array" (`KismetStringLibrary.EqualEqual_StrStr` (`|GetArrayItem` (`JsonFieldData.GetStringArray` (`JsonFieldData.CreateFromString` (`JsonFieldData.GetContentString` (`JsonFieldData.SetStringArray` (`JsonFieldData.Create`) "strings" (`|MakeArray` "one" "two")))) "strings") 1) "two")))

(event `Test_03_Add_Number`
  ;[1 1 1] JSON Types
  (`BlueprintMapLibrary.Map_Add` (`self.Tests`) "Test_02_Add_Number" (== (`JsonFieldData.GetNumber` (`JsonFieldData.CreateFromString` (`JsonFieldData.GetContentString` (`JsonFieldData.SetNumber` (`JsonFieldData.Create`) "number" 42.0))) "number") 42.0)))

(event `Test_08_Add_Array_Number`
  ;[1 1 1] Arrays of JSON Types
  (`BlueprintMapLibrary.Map_Add` (`self.Tests`) "Test_13_Add_Numeric_Array" (== (`|GetArrayItem` (`JsonFieldData.GetNumberArray` (`JsonFieldData.CreateFromString` (`JsonFieldData.GetContentString` (`JsonFieldData.SetNumberArray` (`JsonFieldData.Create`) "numbers" (`|MakeArray` 0.0 42.0)))) "numbers") 1) 42.0)))

(event `Test_04_Add_Object`
  ;[1 1 1] JSON Types
  (`BlueprintMapLibrary.Map_Add` (`self.Tests`) "Test_04_Add_Object" (`KismetSystemLibrary.IsValid` (`JsonFieldData.GetObject` (`JsonFieldData.CreateFromString` (`JsonFieldData.GetContentString` (`JsonFieldData.SetObject` (`JsonFieldData.Create`) "object" (`JsonFieldData.Create`)))) "object"))))

(event `Test_09_Add_Array_Object`
  ;[1 1 1] Arrays of JSON Types
)

(event `Test_POST_TestResults`
  ;[1 1 1] Display Results
)

(event `Test_05_Add_Null`
  ;[1 1 1] JSON Types
  (`BlueprintMapLibrary.Map_Add` (`self.Tests`) "Test_05_Add_Null" (`JsonFieldData.HasKey` (`JsonFieldData.CreateFromString` (`JsonFieldData.GetContentString` (`JsonFieldData.SetObject` (`JsonFieldData.Create`) "nullobject" null))) "nullobject")))

(event `Test_11_Add_UObject`
  ;[1 1 1] UObject, Any
  (`BlueprintMapLibrary.Map_Add` (`self.Tests`) "Test_11_Add_UObject" (`KismetStringLibrary.EqualEqual_StrStr` (`JsonFieldData.GetString` (`JsonFieldData.GetObject` (`JsonFieldData.CreateFromString` (`JsonFieldData.GetContentString` (`JsonFieldData.SetUObject` (`JsonFieldData.Create`) "uobject" self))) "uobject") "DummyString") (`self.DummyString`))))

(event `Test_Async From_File`
  ;[1 1 1] Async
  (bind (_json _bsuccess) (`JSONAsyncAction_RequestFile.AsyncRequestFile` "M:\\Sample.json")
    (:`Completed`
      (if _bsuccess
        (`BlueprintMapLibrary.Map_Add` (`self.Tests`) "Test_LoadFromFile" (`JsonFieldData.HasKey` _json "type"))))))

(event `Test_11_Add_UStruct`
  (bind _returnvalue (`self.K2_GetActorLocation`))
  (bind _returnvalue_2 (`JsonFieldData.GetObject` (`JsonFieldData.CreateFromString` (`JsonFieldData.GetContentString` (`JsonFieldData.SetAnyProperty` (`JsonFieldData.Create`) "location" _returnvalue))) "location"))
  ;[1 1 1] UObject, Any
  (`BlueprintMapLibrary.Map_Add` (`self.Tests`) "Test_12_Add_UStruct" (== _returnvalue (`KismetMathLibrary.MakeVector` (`JsonFieldData.GetNumber` _returnvalue_2 "X") (`JsonFieldData.GetNumber` _returnvalue_2 "Y") (`JsonFieldData.GetNumber` _returnvalue_2 "Z")))))

(event `Test_Async_From_HTTP`
  ;[1 1 1] Async
  (bind _json (`JSONAsyncAction_RequestHttpMessage.AsyncRequestHTTP` "https://www.prevision-meteo.ch/services/json/lat=46.259lng=5.235")
    (:`Completed`
      (`BlueprintMapLibrary.Map_Add` (`self.Tests`) "Test_LoadFromHTTP" (`JsonFieldData.HasKey` _json "city_info")))))

(event `Test_11_Add_UStruct_Array`
  (bind _returnvalue (`self.GetTransform`))
  ;[1 1 1] UObject, Any
  (`BlueprintMapLibrary.Map_Add` (`self.Tests`) "Test_13_Add_UStruct_Array" (== (`JsonFieldData.GetNumber` (`JsonFieldData.GetObject` (`|GetArrayItem` (`JsonFieldData.GetObjectArray` (`JsonFieldData.CreateFromString` (`JsonFieldData.GetContentString` (`JsonFieldData.SetAnyProperty` (`JsonFieldData.Create`) "locations" (`|MakeArray` (struct) _returnvalue)))) "locations") 1) "Scale3D") "X") (.x (.scale _returnvalue)))))

(event `Test_11_Add_Map`
  ;[1 1 1] UObject, Any
  (`BlueprintMapLibrary.Map_Add` (`self.Tests`) "Test_13_Add_Map<Name,Vector>" (== (`JsonFieldData.GetVector` (`JsonFieldData.GetObject` (`JsonFieldData.CreateFromString` (`JsonFieldData.GetContentString` (`JsonFieldData.SetAnyProperty` (`JsonFieldData.Create`) "map" (`self.DummyMap`)))) "map") "One") (1.0 1.0 1.0))))

(event `Test_11_Add_Set`
  ;[1 1 1] UObject, Any
  (`BlueprintMapLibrary.Map_Add` (`self.Tests`) "Test_13_Add_Set<Name>" (`KismetStringLibrary.EqualEqual_StrStr` (`|GetArrayItem` (`JsonFieldData.GetStringArray` (`JsonFieldData.CreateFromString` (`JsonFieldData.GetContentString` (`JsonFieldData.SetAnyProperty` (`JsonFieldData.Create`) "set" (`self.DummySet`)))) "set") 1) "One")))

(event `Test_16_Add_Vector`
  (bind (_returnvalue_x _returnvalue_y _returnvalue_z) (`KismetMathLibrary.BreakVector` (`JsonFieldData.GetVector` (`JsonFieldData.CreateFromString` (`JsonFieldData.GetContentString` (`JsonFieldData.SetVector` (`JsonFieldData.Create`) "v" (0.0 0.0 1.0)))) "v")))
  ;[1 1 1] Vector Rotator Transform Name Color Texture
  (`BlueprintMapLibrary.Map_Add` (`self.Tests`) "Test_16_Add_Vector" (== _returnvalue_z 1.0)))

(event `Test_16_Add_Color`
  (bind _returnvalue_r (break `LinearColor` (`JsonFieldData.GetColor` (`JsonFieldData.CreateFromString` (`JsonFieldData.GetContentString` (`JsonFieldData.SetColor` (`JsonFieldData.Create`) "c" (make `LinearColor` 1.0 0.0 0.0 1.0)))) "c")))
  ;[1 1 1] Vector Rotator Transform Name Color Texture
  (`BlueprintMapLibrary.Map_Add` (`self.Tests`) "Test_16_Add_Color" (== _returnvalue_r 1.0)))

(event `Test_16_Add_Rotator`
  (bind (_returnvalue_roll _returnvalue_pitch _returnvalue_yaw) (`KismetMathLibrary.BreakRotator` (`JsonFieldData.GetRotator` (`JsonFieldData.CreateFromString` (`JsonFieldData.GetContentString` (`JsonFieldData.SetRotator` (`JsonFieldData.Create`) "r" (struct :`Yaw` 1.0)))) "r")))
  ;[1 1 1] Vector Rotator Transform Name Color Texture
  (`BlueprintMapLibrary.Map_Add` (`self.Tests`) "Test_16_Add_Rotator" (== _returnvalue_yaw 1.0)))

(event `Test16_Add_Transform`
  (bind (_returnvalue_location _returnvalue_rotation _returnvalue_scale) (`KismetMathLibrary.BreakTransform` (`JsonFieldData.GetTransform` (`JsonFieldData.CreateFromString` (`JsonFieldData.GetContentString` (`JsonFieldData.SetTransform` (`JsonFieldData.Create`) "t" (`KismetMathLibrary.MakeTransform` (1.0 0.0 0.0) (struct :`Yaw` 1.0) (0.5 0.5 0.5))))) "t")))
  ;[1 1 1] Vector Rotator Transform Name Color Texture
  (`BlueprintMapLibrary.Map_Add` (`self.Tests`) "Test_16_Add_Transform" (and (== _returnvalue_location (1.0 0.0 0.0)) (== _returnvalue_rotation (struct :`Yaw` 1.0)) (== _returnvalue_scale (0.5 0.5 0.5)))))

(event `Test_16_Add_Name`
  ;[1 1 1] Vector Rotator Transform Name Color Texture
  (`BlueprintMapLibrary.Map_Add` (`self.Tests`) "Test_16_Add_Name" (== (`JsonFieldData.GetName` (`JsonFieldData.CreateFromString` (`JsonFieldData.GetContentString` (`JsonFieldData.SetName` (`JsonFieldData.Create`) "n" "UNITTEST"))) "n") "UNITTEST")))

(event `Test_17_Load_Texture`
  (bind _returnvalue (`JsonFieldData.GetTexture` (`JsonFieldData.CreateFromString` (`JsonFieldData.GetContentString` (`JsonFieldData.SetString` (`JsonFieldData.Create`) "texture" " data:image/png;base64,iVBORw0KGgoAAAANSUhEUgAAAMgAAADICAYAAACtWK6eAAAy1ElEQVR4nO29eZwdV3nn/X3Oqbpb327tsmTLuy0bmxi8gDE2lhzCyxICBtNimeRDwjoJGZaZLANh0mqYATwMeSEJ4Q0x2zDDog6BEAbIhMSSwcYsNtjY8iKMZcmyLclq9Xq3qjrP+0fdut0t9Sr1UrdVX32u1Oqurjp1zvM75zxneY6QMStUEegRdu40AHLDrnDS6376Nh97YD0qp+PMJkQ3obIJdCPCepTVoCtQyogUgTyoj2IRMc2HOYQIJECpg1YRRkAGEfpRDoE8ieEAwn7UPY7oE0RnHJKrPh1Mmq5bt3gAbN3qoFdF0AXJqGWGLHUC0oz2YNi6xbB1vYr0Rcf9fPerNlILNmPkEhyXorIZ9CxUTwNZQd4KVuJcVkAVHOA0/lrHff9YcxVAmr+bfG0EzLjvKxAp1CMFBoFDiDwGugcju7HmPgK3R6785hPHpV27LTsPCTu3OuntdfOZb8uJTCDHoNpj2LnTsHOXk15ahqP3defQ8BmoXk3orgGuQPV8CraDnI0vihwECqGLDRd1jDd9TfJbxvJdZigDHS8d1ebvjJeTgBisgGfAF7BxQ0Qjglo0isgjCD8D+SHwI/zcbnlmX2PcXYWdWyxbtzqRTCzjyQTCOAM5pjbVu159Nja6HtUXofp8kPMpe7HJBw4aDiLnEGn+jsb1vYrMaPjz/hIoos02SbT5YgZrDDkDvolLezQE1UcQuQPhe/jeLrn0Hx5r3abVau6Ksm7YKS4Q1R4Du2V890l/fuNmRF+Gulfg5Go6vBIA9SgWBITNXzYwVyFM0pWaK9L6a7aPjPtzLRHjkTOQb7Z6lbCC8mMs3wS+Lc/65kOtX9VuC5foqdyqnJIC0R3dlu6xgtefvnwtOfMKnLwe566n7OcIFWoRRC5CREENNJ3oaW9+jAJkXK8q+SBzNPREWInvomPPmep509/PgThUBWssBQuewEjQQOT7iHwZV/+mXPHdw/Ejegx9u0W2He+HLXdOKYHEwuhzSddB73n5Fah5M8prKHnrcQqVEJQQVFAxM/sITQNNjN+YMRGg4BxEERoGaBiiQQBhiEYhGobxz51D1Y21LkI8oGXij3geYj3wPMTzEd9DPA+sF1+TPEubzxsvoJkEE3fNHIgieBQ9sAKV8BDwNZz5jFz5jbuaryr0dZtTSSinhEC0p8ewHVotxt2v+A0s70T5TUqeoRJC4KJmrZ5Y3BQ3G2d4TQMGARehjQZaq+KqFVylgtYquFoNDRoQBGgUNcUwzoBn7HONtUCSPNPaWCi5HCZfQIpFTKkDUywhhSKSy4GxtASaiCZJ9zRZBepQwDOWDg9GQ8XwfxA+IZd983txFvTEQ92nQNdrWQtEQbh1i03mLPSnv/XreOY/48mL4i5FCBDGcxCzFIW1sYaiEK1ViYaHcEODRCPDaKWCBo1YCCjQNOoJ3Stm2Q2aJh3julma+OUIYi3i55BiCdvZielagS13IcVi3Npo3JrNSiyKxnMxeHR48ahcqN8D92F59j/9GzTnVm7YFcnJe1apZdkKRLXHtFqMO19xCQXpxcprmn3tePhVxM5wk4miCBpEw0NE/UeIBvpxoyNxlwkFMUjSvTrW8I71E+aLyZ6jijrXHGEWxPcxHWXsylXY1WuxnV3g5yaKZcZumEaAUPYNkULkvkbEn8sV39wd/3gsr5cby1IgeusWT27YFeqO7hyb6+/FyJ+QtyWGGnMThueBc7jhIcJDBwmPHEYro6iLYh/B2onGtVBCmCvHpimK4sl5Y5FSB96adXjrT8N0dsVdtjCcm1C6coZaWEW5mV2Nj8i7vltP8nxB32sJWFYCGe9E6o9f/hwK5lMU/SsZaoDTaE7CCEPCpw8RPHkAN3AUjULE2HFOOOkRxEyMT69zscCth1m5Cn/jGXhr17feedZCMWLpysFoeDdB+PvynP/z42MHQZYDy0Yg2oNhOyqC6k9f/k5y9qNYk6MShjCDjwGxYTRbjPDgkwSPP0Y0NBQ7x0lL0S6CmInmu2izi2U7u/DPPBvvtI1jLcpsRr8gouR5RK5BGP2xXPGtv1RF2I6MX4XQziwLgSR9YL11i8fKFf8fZf/NJ9JqRP1HaPxqD9HA0difsHbsmuVIIoIoQp3DrlxF7rwLsavXzLU1MXTlhJHGZxkYervcsCtcLn6Jt9QJmDM9PYbdl7ZK7W2rvmdEPhD84JY3dTa6jnwtV/ZfFB5thCBWROy0jb3SHN1RGnv2EOzfi6oiXj7+uRs3MbEcSV7P+GAgGhwi+Nnd+GedQ+7cC+LFkVE0w+uL1QjlaBB6q/JvCtzKM39wy5tuEvnA8Nve9jb/00d/Y0wkl9yvtNnCyPYo+Z4eswXMrt7eyZeYK2UefPF3KeWvZbARAP6s7msEqlXYfS8c6Qc/qS+WaYsxI01zCEJYsxouuQyKxXEVxUxowIq8T6V+Oxf/80tEGJnsqi09Pd4ucO0glpQLRIXuPkPfttbM7QX/4YubXNQ4R8JwrbWabwSq77vmgd+/4Ay3dXQgCIzBT+YFZrg3IDT2PYobGkT8XDybnYGIQYMGpmsFubPOZS75GUUallflvF8eMDs/9MNnfCrni0SR1NXznjY2t/eXf/U7j7d+pXuHpa/btRZXppD0CqR7h02Ece5bPr3Z+PYNqPtNVX2GWK9DjCVJfiNwjFacMxYz+9q/uTzD2NjfUE1zbiwuCojE8ykuHtmdS766CNdRMibnJ0vXFHURGoWjIvIAyLdd6P73o7e87WFgQlmnjXSaRDPDzn3zx08zuXIPyu8av1B0UYBGATinyNgoiYAYYeaFhFORieN4miI5UZzG28LG3c9gjIj1MdbHBbUqyBdcMLz90c+8+2BaRZI+s+jp8ejtDc95y9+82PiFW4yX2+TqFVRdKLQWD6Yv3RmzQdF4rl9EPJPvwIWNx6NG462Pfebffzcp+6VO5HjSZWhbejx29YbnveVTvyu5/GdRFRcGocRDtelKa8bJoqoaGc/3EFFt1N/0q1t+//OJDSx14hLSY3TNJva8N3/y1VLo+JoGgUMjWoEMMpYnqg6xiJ8zWhu56Vefecc/pKm7lQ7j6+kx9HW78//g7y7AL3xBozATx6mCiEEjNAocfv4L57/57y6gr9vR05OKsk9FImJEtRF+ynh+WaPQZeI4hRAxGoXOeLmySvipNA37Ln0Xq9mcnv+Wv3mx5Du+64JqBDMsD8lYpmhk/KIN66Mv2XvLH/xzGrpaS19LX9KtAM6Yd8V7v9NTe2QsNqKIqGDeBbRsYylZWoH09Bh6xV349k+dIchWF9QEyFqPUxfrgpqIka2b3v6pM+iVJfdFllYgO+Pnh9hrTK5YRFvTthmnJoK6yOSKRR97DdCykaViSR++ZWvzC6fPQgyqWffqVEdVFDGxTTDORpaIJRXIrp3NL4RNp+4K2ozjURDdBONsZIlY2i7W+kuTMB0lZrE3J2P5I61A31IExtnI0rA0G6ZUpbsPc+j+nT49t8r+p/Y0xMRLrDKRnNqoxitPxUiwpedWD/DW71D6unHxKOfisrgCaQqjTyTqg4j4w6bf/otf+CZHFNTjOFIZpyyqitocwejIL3b13hCSxEIGuneoXWyhLJo1du9Q27dNIoA3fGtgVRj41ynhc8W5M6sjQxdXKyNXE4W66FHRM9KFolhPiqXyj4rlrgfVmP2e9X4c1oLb+7at7IeJtrTQLIoxJi/0qi/u3eh3rf0jUX2D9QsbpLkfXKMQF9bnti8nY3mS7GPzcoj1441bUUgU1J5SlS8HrvLRr9+0/snFEsmCCyR5ke4dT7/G5kt/ZQvFDWFlGBcFUXI4jM42cnrGKYQ6oXlkgyDG+tYrdRJWKwddVP3DvpvW/v1iiGRBBZK8wE19T78z37HiE1GjRhTUQ0Fs5mxkzAlVVTSyft6zuSLBSP+7+7at/8RCi2TBjHSs5Tj0Wr9zzVfCylDknBPJVulmnASq6owx6pW6bDB85HV929Z/dSFFsiDG2tOjpq8b99ovHzlT/MKnw3rFZeLImA9ExDjnJKxXnPiFT7/2y0fO7OvG9fTogtjWgtx096UIIhpZtvulzi7XqLtMHBnzhYgY16g7v9TZ5TzpQUR3X7owvaH5N9qeHtO3TaLXfePw6WLM64KRQRWT7e/ImF/EiA1GBxWR17/uS4dP79sm0UKs/J33G27Zut0ARIG8JNexoqQudNkikoz5R0Sj0OU6VpRc3nsxjNnefLKQ3Z5rsg1QGQtLvMFKXfT8hXrCvAtk69YkoJs5Ow5llc2MZywQgqgLBeRsGG9788f8tyDbm/8KRZ110OOMjBNDnYI0V/5un//7ZyNLGRnTkAkkI2MaTkogCqI68XPppX2imvkdGYvLeNub8DnJ1SInJBBVRG/d4gnxmYDjP9u2vTYSoZm2jIyFR5EJtjfhA6q3bvFOtNKe84Yp7cGI4CA+8le//qyV+K718KHGetOVO+ReXwv85Xq0X0Z6UAWPwNdv/dqqxPZaPwyMyqvuGUiOp9YezFwPF52TQJIH6Oees4HV7j+ivJSQDUQYmgotMwhVOI+HO+9rXEkRtS7rcWUsAAa1lUbEM/Xhq6jySGx7ufiH8VHUTr9x5VOI+S5D7i/kd+56cq4imbVAWuL42pVX4Ok/UvQ2UXNgJzYTpnl8h+fcsj0cNiM9qIJnnIeRVWayitjIWgrmmaCv1x1XvFK23X3XXEQyK4E0+2+qlz5vNRL8I57ZxFDYADyO6ds5wKBoNkGYsUioAqGqQzHHbkmNVGm4kKI9g0i/oTue9yy67zyq2xGRmfevzs5J37nFxjcL/oCyt4lKEAA54gZjwh9JvkohQnywrRGwx3yS76cy4YtEW+fPeNsb/ye28RyVIKDsbcIEfyCCsnPLrBbQzq6LtXVX1EzEy2g4bZejCYSxZZJOIXAQOiVSjuv+JUbhGcEz8f+VOZyA3KYkRu8UwnH5c+x7yyT5A3E+tkUWiRgaTlFeBvxXdu6any6WEjdFqghfYw0OSfvq3KTwAgf1IN74XvKF9R2GtSXD6oKhMyfkbFy4tRCGGo7+quPwqONoTamFijVQsLFBOI4XVbsiEleroYPRUIkcFDxhVUFY12FZXTR05QwFLxZPI4LhhtJfczxdcRypOoYbcd867wnJYbbprkxEYttlbcufjrNi2lTPZRRLjvU30kYijGqghArrOwy/tinHs07zuHC1x2kdhrw3/SuMBsoTwxEPHgn5+VMBDzwdMlBT8l4slnYWSiKMWqTUQ1hZEC47zefZp/lcvNbj9E5Lhz99/tQj5eCIY09/yD0HQ+47HHBw1OEJFJu/m26hEK/Z6p3dpUsTWXGeSfrOlWZrcck6j984N89zT8/RlZ9Y4Mrk3YLkHh2+cOHqWFC/dWGBg6OO2/c3+NdH6+wdiMh7Qt5ClHYjOAYrUI+gHirnrLT8+rl5rjszx2kdx/eW3RT5IwJ5K5y1wnLWCssLz80zVFd+8kSDf3m0zu7DISJQ8mTSe7QjbS8QIxA5GGkol6zz6L6kyHNP91s/T2ozaf4l476egI79kwjIAKd1GF59cYHfvDDPv+1t8A8P1DgwHNHZFF7aW5OkMzxYV87oNLz64hK/fm6OvB1Lv2NMAIlXO13+MM74u/LCC8/N88Jz8/z4iYC+3VXuPxzS4QvWtEFrMgOzG+YF4S5SdxSzNTDaUEq+8PYrS7z8wkLLudZmBzPpduFcXFrWTv4W0vwl5zAy5oUmBpS3wkvPj2vdr9xf5Vt7alhJd2tiJPYfIlVuvKjA659ZpDMXv1eksRBEmicWOUWdA2MmdzGb35IoAhHExC3P+Lx+7uk+V230+daeGl++r8pooHT4krb8Ee7CzraBm3k0qgcroHIVAUhqzq+2AoM1ZfMaj//+wi5esTkWh9Ox7lKrmJOCt3bs/06b/477iCDWxr/smjHLmqM3EBtVZ0546+Ul/ssLOlmRF0YDbf08Tdhml3NFXvgvL+jkbVeU6MyNGasdP9TiHJjmu4scny9JXkGch8aM5Q8TR8KMwCs2F7j5hV1sXuMxWE9b/kgoVxEIKD0zn2Y2ZQuiirAdkV7C+3rIXbCu/FIkXEvkK0scQddK3GV44bk5/sNzOsjZuOCT8foJqIIx1O66l6G+b9HY8yjaCMbF2QcQUMV0FMlfdgkr/t2r8M/eNCascc9Nhn6v2uhz8wu7uPmOER46Ek4wvqXGSjzqdNEajz99fpn1HSZuMcaJvUXzHYPHHmfwS9+gfs9u3Ghl0vyRnE/ugnPp6n45hasuG2s6mphxFclZKywfuqGTv/7JKN97tMGK/BLnjyJEKBKurX2yfOO+B0e+I73UtQfD9nhh42S/NqmZj5+Kr3y89EZr5U9zvnkGq88Bm5+24x1rp86f80l+znMoMYqbx20niThedXGBt15eAsZqruNoFn7/X32W/r/8LIQRkvOnHqV2Dm00MCtXsP5D/5nyy379OJEkJIKsBsqHbh/h7qcCulIgEisw1FCu2ODzvuvKFL2xyuM4mu828p1/49B7P4IbGERyuUnfF4jjKAcBGMPqd76Z1e9805T5M75M/u5nFb7+YG3eRWJwVOjg2fyED/AOlDzTTo6LQFSH/r00Qvdg4PTm8jsrn4epFzIe14IkFw58eMWqYjm8JZc3r44CZaSqUclhzRIG8EnE8cqLYnEkA9nTiWPwS9/gyEc+iV2/FjESb9GcMhMF01VGa3UOvmc73sb1FC5/5qRGYJvduaIvvP+6MttvG+a+QyHlJRSJlXiw4rL1Hu9/QZm8jUeTphNH7Wf3cfDd28H3sGtXo5Fj2vwxJdQpR27+JHbtala84cZJ82e8L/jWy0s4B//48PyLZK5EDqpVjQq+XNxRMJ+r/nXHK+rD3pvlvYNHJxPJhLdKLjh8c/H0QjnamSuYV4+MalgNcCJLe/psUjNed1aOt18xJo7Jm8C4W+UGhzj6N5/HrloRfzuMxvWpJ/s4NAghn0ejiP5PfGbaNCU+T94T3nttJ5u6LNVQJxfsAmMEqqGyqcvy3ms7W+KYKS39H78FjSIkn4/ffab8CeNFFXbVCo7+zedxg0OxOCbpVSQjY07h7VeWuO6sHEONpfVJmmmytRA3MqphIW9eVShHOw/fXDxdenHaM1ETrf8kG0r0E6u7Oor2O/mcXDYyooEInizx1lwjUAuVs7ss73puB8q44drJaDqQ1Z/eS/jkIcjlxpzM2RCGmI4S9XsfIDzw1JQGkKTNaTzc+SfPL+ObuIZcTBsQ4i6fb+I0dOVnEEezAgkPPEXtFw9iOkoQzmH8xTnI5QifPET1p/eOfW+KtCXezLue28HZXZbaElUix6TLiOCNjGiQz8ll5aL9jn5idReMaQHGG35f3HqMRPUvFIty2UhFAxH8Se696KgCIrzz6g46fDnWNzz++ua/4ZOHIDrB3SgiuGqV8PCRcYmYHCOxgZ670vJ7zy4x2lhcAzASD3f/3rNLnLvSthzyKWm+S3j4CFqtndDKIQGIXJzHTD9mKrGPT4cflyHxltNUIII/UtGgUJTLRrT+BenF0TemCwOgO7CyjWjo/y2/tdxpbhwdSY84khGZV2wucPEab+bCH8/JlkLSiZ4FiU/ysgvyXLHBZzRYHJEYiZfHXLHR56UX5Kf2OSZDdR7yaHa/n1QiF6/xeOXmAsNL3NUajwj+6IgG5Q5z49DHym+VbUS6I3YpTE8Phm7c0CfK66zRj9Rr6nSJ/Y0EIZ7o2lg2bHtGIe4ZpCRTp+ONzypizeLUkqpgjfDGy4rpmsWdBNNsSbqfUWBjp6ERpWfmWQVbr6mznn5k6BPldXTjenowZnvcF1Nx+kelklndCHFL7XMkJI7nKy8q0JGT1pKItJL4Ixeu9rh208K3Iknrce0mnwtXe7NyypcSIV6V0JETXrG5sGQDGpMhYBohrlQyq0X1P4mg28EY6SUc+FjXaiO8tV5VTVYeLDUCNBxsKBteeG4+XhuVksycDb+1uYC3wK1IvN00nrluF5Lh3xeek2dD2dBw6an0BGy9qmrgbQMf61otvYQGwDPuplKHWdWIcJKS3YCmOQl37Zm5Mcd8qRM1CxIDuGiNxyXrvAWrJZPW9ZJ1PpvXeG1TgSRL3so54dozc1QXyVebDSJII8KVOswqz3OvhqQrJWwjQlOSTqA5v2DhBWfmljopcyZZwXrtmTnCBaohhXjD03XN/GnHVbPXnZkjb9OV9nh0DsXxWgAz+qniGap6db2hgqTD9xCBRhRPep23Kp7sT0stMxuSTLx8g7dga7SShZOXb/AmPLMdSMry/FUem7osjUjTs0dVMPWGiqJXj36seIZxNXNdKSedgcNNNTG92Bji0atnrPXi7a4pqmFmQ1LYGzssm7os9Xk2AJF4Z9+ZXZYNHXbCM9sF1/SfLl7r0YjSI3ABCRyulJNO55lrjSLXmHiZaqrMUIHNa7zW1+1G1JzMPH+VRzjPBmCAMILzVnnx+rs2zKAkyYn/lCoUNVYQlWuMEX4tPmMhHa0HJBuU4MyuZu24tMk5Kc5eaRfEALR573YlKdOzumzshyxpao5BEHWKg8uMoueE8QLO1Nihc3EUkjXFZAyh/UjSvKHDYM38toJKvJtyQ0f758+aoqHoy5yWyi04isSDK3qOEVgTpeiYzWThXck3dDS3h7alBTRZkRf8eZ4P0ebCxBX5Ns6YZtI7ckLJX/wFntMhEi+LF1hjFOkYt3ty6RFQjcPs5JrDHelI2NxI0lzw47ha892CeGYszE47549vhIInsQucnhcR50BVOoyAlzYnKZn0SkurdjIke7/nWyBTbhRrM5KQpmlZ3ZugAII1qkRpy2ehGZspZZl2IiTvMZ95nMxGt9vw92Qk75FGGxSIDGglVTW1gojQiCBoWkA72kGS5lrIvM+mJ7PotXDis9qJJM2BU+pRXOZpepE4ZoVWDEi/F2+YS03ykiiJlaCZpNSkbO4M1R2Bm/+JwtApQ/U0Df3MkWaZjjbLOU3dRVXUM6Ai/UZEH/PikHCpMENlLKZTf9W1vtduJGk+OOqSEZF5I2lBDo22f/70Vx3VZmyx1LyHoJ4F0H1GlfvEpGsm3TSXUjw+HAcISE3CToB9g9GC3fuxBbz3QpOU6eNDjnqK9oUAoGhTE/cZUb1T451IaUoiqvDwkfY1gKTAHzka4i/AMK9v4nuPf1Y7sqc/TF8FKIg6ENU7jfX8H1TqruIZjKaksnZAzsIDT4dz22OdEpJRq8MVx76hiFwz2vl84RRynrBvKOJwxbVGtdqJZA//A0+H5FK01ERBPYOp1F0l8PwfmOI7Bx9VuLvgi6LpSKdqHCx632DU6ka005Bmkok/PxgwWFNmOJLkhPAkjk18z8FgwjPbgaQsHxuM2DcYkbfpiXKC4gq+KMJdq945+GiymOfv8ZC0OOowtmPujv0NICVN2yxJVu7evr8x7+uwEpL1WD9o5k9alovPhiQ/bt/fSNW+dCAerPIQdXwNkqMgPP1qtaKjnpl9WPiFxml8LNht+xutQGOpSNgMOAUkrh1/cSikOM/dq/HPKXrCLw6FcSsr7dHKJqskaqHy/f0NCguUPyeCgnqCrVR0VHL6VQCjO7DlP6w8FTn9YqEggpIKz1iJl7zvH4z4/r5Ga3a9HRDgW3tq1Bb4aATbNLRv7amla4RlGpJZ8+/va7B/MCJvU1TxKVGhKOKcfrH8h5WndAfWcH98QKeV6MO1mo56FpOWSUNHHPf26w/VqIfaCmGZVpKwO/uHInbubdCxwIGsI42jFe7c22D/UNQKO5RWmo0r9Uj5+kM18p6kxndSRT2LqdV01Er0YVWE+1GThFosvbu2L4jcBwslMUAqDspRhYKFvQMR33y41hYGAPA/760uWt868dX+573VCWlII0kF8s2HauwdiCjYVI2+hYWSmCBwHyy9u7YvCcUb+3bbcLoD2zlQ+ejoiLutXBLfaTpEEjVDxPQ9UGPfUNQaHpwVi9jvSM7guG1fgzseb1DOLU7f2jXz547HG9y2r4Gd6xbcRcqjZLh+31DEjgdqS3pMxLE4JSyXxK+Mutu+e2flf+gOLNvixi05r1G5H6UXxenr6g3dVy6IlxaRGIlPZ/3LH4/OagFjUuZ27Row5sRqVVWkkMeuWTXjpUnhHxx1/O3dFYre4g5batNh/9u7KxwcdbOuROyaVUh++gORpnwmgDHYdWuA6XU2fmHiX/54NFUz504JywXx6g3dV6m513f34bgfTcaEWqOD0oujByn/x8qTIyEvCULd31kST5VgqX0Sp/EW3N2HQ/727srMXa3mYS7Fqy6LDTwM57a5xFq0WiN/0fn4mza2jguYjCTSfD1SPnrHCMN1N+8bpGYi2UA1XHd89I6RVhSVKe2+eZyDv2kjuYvOjyO82znsbxeBMMSuXUXxqsvG7jkFSdfqb++usLt5Au5Sd5VVUVWCzpJ4QaSPN0Jesu5Pq0/Qg4w/RGfCW0lv3NVa+56RB/pHgusbgbu9XBbft4gusV8Sabx99dt76nzl/mqrKzFpPjcPorRrV7PyTa8lero/PqDSNk9wneYjnoUoQoOQVe/43WnPBtHE61T4iztHeeDI0hW+azrsDxwJ+Ys7R1se8ZQiaYp+9TveGB+rFkXxu8+QP1iDWEv0dD8rf++12LWrWwegHvcIxrqeX7m/yrf31Jf8hKlmukLfIuWy+PWGu6MyHLyg6z0jD+gO7LQnTAHINiLtxm58b33vHYdHt1Zr+j6EQ+WSeEvdLEYaH1TzxV9U6XugFq8AnWpjVfMk1lVv/21WvuUNhE/344ZH0SBAg3DyT6NBdHQIrdZY94E/onT91dOewZfU0h+7c4Tv72ss+RmFkUJXTvj+vgb/486RVus2qWCb+VO6/nms+8Afo9Va/O6NxtT5EwS44VHCp4+w8s2vZ9Xbf7spjuPzJykXK9D3QI0v/qJKVwrEYQTKJfFEOFSv6ft++PTollXvre9NjgA59vpJT7mVPqLmcWwhjHx46BPlW0xDX2ON/ZAxrGjeZknk4jSOKPi5n1cYrjve9Oz4IM9JD6ps1v7rPvBHFJ9/JUM7vkWwd3981NgkmGKB/CUXsuKN3VOeTTj+WaMN5WN3jnDngSAVNWOSthV54da9DarBMP/peeXWcPOk+eMcK37nJvLPvIjBL/RR370HV61Nem/xPfxzNtHV/VuUX3rDWP9ykjRYiQ3ks/dU+PvdtdapV0uIYsAZO9gI9M8CR1/Xu0YOA/HRg5OIA2YwcgWhBxsLBbTvygfJm4toOMcUqxsW+pTbBCMwVFeu2ZTjHVeVWF00rQKY9CjoZkG6ShWC8Pg3V5BCHsk3YwFPIo7xxwv8sj/k4z8eZe9AlKojoBOSg4fOWRkfW3fh6rgunPSIhHHvqvUGWqtPmj/4HqZUbP7/eHGMz/+jVcdf/7TCDx9vLJg45njKrSNnDHX3kHTfdTGA9uDRSzTdIo0pz0mHZhe2l0gVoQ+flByNAHFhrMgLPzrQ4NGBkDc9u3RcIOeWIbTiuMhYAU9542YXNDEYxmzBSLxR6R8fqvGV3VWCSFMpDhiL3fv4UMT7bh3mdZcUeeVFhdYAQvJOAq2WBEDyubFKYjKSTfbWTPgWjOX39/c1+Nw9FQ6NutS0rOOwuoMc3QTI9OKAGQSSIIKqEvL36ZqHSoxgoKZ85PYRnrcpx7ZnFFohS5NrBBBrmqeUzvAKxkzwa8ZHV/nRgYCv7q7y4NMhHbk4XE3KCn8CUXM9m1P4zM8r3P54g9deUuTqM/zWOyXGLWKSfdjT39QISjyMrcQtVSKMh4+E7Nhd484DDXJW0lp5KN2EMssTNWYlkDQTKfgWclb40eMNfvZkwFWn+7z4/DyXrffxjunduWkaYSHuN44/Xno0UH7yRMA/P1Lj/sMhIrRqxaUeqpwNSRpX5IVHjob8tx8Mc+k6j//nvALPPd0fC86XXD+b/GGs0ggd3Hso4P8+UucnTwQ0IqWck9YIVrvT9gIBWrVZRy6uFm7f3+CHjzc4Z6Xl8g0+zz7N59yVlpUFM+MElWq80WlPf8jPngq452DAkyMOI/FcDLRnwUfNyUSA3YdD7j00wsay4dmn+Vy+weeC1R7rSzPnD8BAzfHoQMQ9BwPufipg70DUGmb27ZI74/PKXASS+tdOCqbcrBX3D0b8sj/i6w/WWFkwnNZh2FC2rCkKnXkTryTVeEXsUF05XHE8Neo4NBoxVNfmimJp3a/dCz5JfxKRsb+qfOeROt99pE5XXljfYdnQYVhXMnTl4y5kPAkaT0IeqSpPjUQcHHUM1Byhi3d+JhVH28Qy2z77S2cUiMSRQEUE1T4diFvgdB+IlhhCzhMKXqzsSqA83B+2tvFOhpF4Rto3sSiSJfbtLoxjSd7HN3HXFCCIYO9AyC/7p35fE88T4ps4nq4Qr7huj/xRbdrugPTiEpue6bdm14Ls3GJhV4jyb+TMc6g5R0qOip4OVVqD21bAa3YxppK2MjbC0x6FfnIk7wqxT5H3hALT5w+0af6oOPLGUnP/CozZ9AzMboJi5y6nikD0V4xGA+SNjxI0QwVN+OjY16lCGWsNoik+bdNFWCB0FvnjNIWFGzPe9sY+8Z+AvPEZiQbQ8K9VEXbumtVWlFkJJF6f0iOy7Z4DhLoN0WE6rY8nwjF/TPJVRsZiMt72xv/xROi0PjBCpK+VbfccgB45ds3VVMx6iluk16n2GNl2178wED6PuvsS6FNAgOKSj2v+m96KJmO5oXFL0bK91gcC0KdouC8z0niedN/1f3VHtxXpnfVGxjnX9KoYae6U1G8/t4tatA4XtYRWdyWTNxX3O3z7y0F+7ZWuPhyBpN5fyWhHNDL5TuvXn77ri7zs9YnttX5srKNgD8vLfjwEE213tsx5HkQEpz0YLu0WeVnfEDA02XU3fa00mpP2iteU0X4YgaqURuWmn++Z6hrd0W25v0/nKg44wYnCuP/WFw+cbZ/YCu2kx2yl121T106hmjLaGKPOaA8msb0JP9yOivSdcKSekzJiEVR6ceM/O9nuZusAZWTMF+Ntb8LnJIMhZrV8RsY0ZALJyJiGTCAZGdOQCSQjYxoygWRkTEMmkIyMacgEkpExDZlAMjKmIRNIRsY0ZALJyJiGZRG0AZrLkuXkNgK3Yu1Oe9Hc4mCfas/T5l/LZa9DWwskCT/jFAIHkeoJ7wgUEWSWlqHN0OAnw3J9nghYETwTr7TVNhdLWwokKea6i0PM5K2yuiiszBvydu7NiACRc4RBMKvrjTF4vj+3hyRocnpASBSFrejwUyZMwVqL53mzawGmIAwCnJvdGlLP97HGzt2wNT4GYqCuDNaVSigYgbzR5MdtR9sJxAjUo9hKzukIecaKBud1Rlx+7jo6Cx5zPS5HAc8Yjg6PsP/JgRkNwzlHuVTknDNWnFAtqwqeNTxxuJ/DRwfwrJ2y1ROBMIpYt2olp69bQRi5E+r+iAh7DxxkpFLFTHOOR1xRRJy5cT2rOjsInZuzHh3CcC3kZ48e5tFhw+6hPI+NxGaWt9p2wR7aRiBJQVVC4ZxyyNb1Vc7vDPBwYCzF5rkc4RwLQIk3dTUcNFwcqmV6gUjz2hML8KAKTsae56Y5w0MEwnHPCyc/hmNGZNzzphuViQVyzPPm+Cwjcdyt04shp+cjrl5b55Fhn52Hiuwd8Sja9mpN2kIgSfyl0Am/saHK9eureKLUnFB3gt+MkZuExTyR+4//zPbaE2W2zzv2uhN97mI/L9JYjEEoGAObOxucVw647VCRWw8W8YxiaA+RpH6YNxGHqvCas0Z50cYKoUI1ikOnGDl5g82YX5LySMqmGgmhwos2Vug+awTVeO9rO5RZ6gUCcctx45mjXLG6xnAwJoyM9iARynAgXL66zo1njhK69ijAVAvESFz7vGB9jSub4jjulKSMtsFKLJIrV9d4wfoa1UhSX9GlViBCPFq1qRSx9bQKlTATx3LASjzQsvW0CptKEfUo3VEG0yuQZsig69dXyZv2Gx7MmBqn8dzI9eursS+SYoWkUiACNCLhjGLE5s4GtTZoijNmjxGoRcLmzgZnFCMaKW5F0ikQgUDhoq4GhTacXMqYGadQsMpFXQ2CeVxvNt+kUiCq4Auc3RHGZwymNPMyThyReL7k7I4Qf5rJ0qUmlQKJgJLnWJ2LiDRTx3IlUmF1LqLkuckPKU8BqRNIcqpT0Wqre5VJZPmRlHPBKsUUl3PqBAKAxkehWWmP5QgZJ4bSPPkrxetO0ikQUn2SUcY8kpz8lVZSKZBkGLDhsuHd5Uy8dYFUD+OnTiBKnHGVyDAUGKxo1pIsQ+LulTIUWipNgaSxnFMnEBirWQ5UbOyHpDHnMk4K1dj/eKJiqWctyNwRgYeHc6kd3cg4OZJRrIeGc6me50qlQJK1Or8a8Xii6pOzWTdrOaFAzipPVD0eHfFSvdYulQKBsb3ntx8uZN2sZUbSvbr9cJFGirtXkGKBOIWip9w7kOP+wTwlT4kykbQ9kULJU+4fzHPvQI6Cl97WA1IsECCeMBTlnw6UOFy3FG0mknYmWSFxuG75pwMlPEn/ZFeqBRKH5IGRwPClvZ0MBJZSJpK2JGqKYzCwfGlvJyOBwTOp10e6BQK0AsMdrlk+90gX+yo+nZ5rjYKkPYNPZZJZcgE6Pce+is9nH+nicM22TYystgj7k4hkIDB8/ledvGB9jeetqdHhORrR2DWRzt2ZV0A0/n2n8dfTxsXSE38WxL8z/nlumvsklUDyvOgEh7zH32e6l5uP542vuHyJR6tGQ8P3Dnbw/UMFQpW2EQe0iUAgznS/Oav+L08WuedojitWN7ios866IpRzgj3R1Y1GCHOx8+iZ6YeUI6d0+Eo539wTPFeaK/TKPox6im+njicsAoEoZR9KOYFo7mFVATBCh684T7HT9BkECJ1SzjWfdyKRR4wQhYIncKhheXg4z139OQ7VLAWr+NI+4oA2EgiM2X7JU442DN95oshtXoH1hYjz+uus6zAUvbkXqhGhWleGhkszBnhWVXKDPitH6yc89GxEGB41jFZLmBme51TpGDV09tdxJxFQemAwRyOYOYC1qnJfXSnmT+x51VA5POp4tL+TgzXDaCjkjFJqjla1kTaANhNIglPwBPzm0O/+UY9fDQVxF+kEKj3V2GiN6ZixAKV5feRqJzwDrBoHwDYyu+c5VZyrntTzrMkhkpvd85zi9MSeF+cl+NbiGaXDi1vIdmo1xtOWAoG4JtJmHzlnlLw9uY3/c40Ye7JhBhb/eXOz0JN5Xlw2mvql7LOhbQUynkQsGRnzTeqHeTMylpJMIBkZ05AJJCNjGjKBZGRMQyaQjIxpONGxPKFHpfvSPjl0/7oJ91jPOnOIw27dM39tp1/ovDasD0eo2HlIa3pI8xa46VhuQ32ikZfvtEFt+PbD9/1ia2J74y9Zf+lh7bu/W+mVGRbaTM7chnl7eswWtppdvTeE9Ir2TXPptm8MBsbzMIHHcts0Gx+THNE+76WIWCTNO5NOCMV4Hsb3g129N4QzXb2l51ZvFzsdvb2zXiQ06xzr3rHD9m3bFi8N7Okx13W+7ALFnS2hW6E4EwcMtagTMaKua/3GD/iF8sVRUHUgy6crp4qXy5MvlnBRlP7WRBVjLfVqhbBRT39654Q66xdNUBt5cOjQk3/uVIwY1cQWBeOMZwbDKNp3R+XaPfSKg2NseQZmkVsq8ZJX0Ws++K9nm0LxrYLcqM5dZP28R+tY4eRWcSsW1Sq4KERE5jyLm14EUIyxrDnjHIrlLlwYptfoNK5hqyNDHDmwF+eSVm95lIcgqCrGethCqfXdmOY7OkcU1CLEPGSs+XqjUb3lR++9YS+qzcUCMm1mzLRyTZD4Bs+/+Y4/Ntb8mc0VV7igjgvqKOqmsn4RMU11LC8E1DlEJN0iOUYcqoqYNtihNFfixXGqqpN3mwQRxBg/h/ELRI3qIC780A/+5Lr/Dkyw8aluPzmqwvbt8pL+q/3hM1f+L7/Y+ZqgMoS6KBTBNC0iZVaxeKhqekUymTjSkralQWMV4cRYzy91EVSGvtZZGPx33+3/UcD27TqVSKbyDaS7r8+wfbsOn9H5Fb/U9Zpg5GiAi1REvKZPcUrnuEjcvB85sJfqyBDG89IxSpSJYzIExIiIh4s0GDka+B0rbhqudn6V7du1u69vSnueVCDdO3aYvm3boms/fNv7/fKqG4OR/gYifpbTE0mdSDJxzIyIIOIHI/0Nv7zqldd++Lb3923bFnXv2DGpFo7PvR419Ipef/POC5zk71NVi4YmPf2HtCGopsAnmVQcKT5XYMlRRTwnhsi4xjNv+9Otv6RHJRnpSjhONVvYaQCN1L7HFko51fAEtyGdKujStyRTthyZOKZGRDVUm+/IRWrfA2jT9ideNfG/KiB62Ud/3lEOh35pPH+DRqEjW5IyK5bEcc+6VSeDE+sbFzaeGvGqF9z7xy8eTTSQXDDB8Lu7+wxAORi4zPr5DRoGeuw1GVOz6C1JJo6TxWjYUOvnN5SD/GUwpoHWBeP/c+iSeF2VGLvZ+HlUJK1nK6YWEbM4IpnS58iYCyoSGT+PIJthTAMJU+XoqsztOFEWwSfJfI75Jbb1VZP9aFKBqGbqOFkWTCRZt2pBULGznwfJmB+OE4k9SZE01x1l4lg8MoEsMBN8ktGTaEmSlmM08zkWkyyHF5x58Ekyn2PJyASySJywSDKfY0mZXCCZbBaEOfskmc+x5Ey+QMtpJpEFYmqfZLxQNPM5FhlhcpuffJgXl5XEgjHRJ6kMDWA8HzG2udBUEGMxnk9laCDzORaLKYIRL4vYvO2ISHx075EnHqM2OkSpaxWenwMgDBpUho4yOngUSa7NWFBUJz8MZQqByIwRIjLmAYmrrZGBI4wO9sc+CeCiMN5rbZZXtKR0M7nNTy4QMSOp2B13ipA46+ripW8iJg7Rk5XB4hCfozEy2Y8m90HEHVbnQE/tbbWLRksI47b5Z+JYHBRR51Dh8GQ/niCQrWx1AEaDPVGjonFwhoyM5YsIJmpU1GiwB8Y0kDBBAL294lAVr2oewrmHTK6gCpk/krEsUQhNrqCoe8irmodQld5jttwe54N092H6em8Ir/3I9z9oc8X/rWFgXBRG08UOyshoO1TFWM+zuSKuUfvgrt4bwu5L1fbFYRlbTO5jxIEb3DUf3vkumyu+3xhvrRjvFA/0k7FsUFAX4qLoiDaq//X29235eE+PmmNbD5jO5Ht6DL297rr/9u115NdcjbqznIvyTDFenJHRFohRY2wdMfuo13/0gz+7/nBi63O+V/eOHdlAfMayZiYbn7k1UJXuPsyh+3dmLUfGsmH9pVu1rxuX+dYZGRkZGRkZGYvO/w+ixYun3iCRswAAAABJRU5ErkJggg=="))) "Texture"))
  ;[1 1 1] Vector Rotator Transform Name Color Texture
  (`BillboardComponent.SetSprite` (`self.Billboard`) _returnvalue)
  (`BlueprintMapLibrary.Map_Add` (`self.Tests`) "Test_16_LoadTexture" (`KismetSystemLibrary.IsValid` _returnvalue)))

(event `Test_17_Copy_JSON`
  ;[1 1 1] Vector Rotator Transform Name Color Texture
  (bind _returnvalue (`JsonFieldData.Copy` (`JsonFieldData.SetObject` (`JsonFieldData.CreateFromString` "{\"copy\":1}") "obj" (`JsonFieldData.CreateFromString` "{\"property\": \"value\"}"))))
  (`BlueprintMapLibrary.Map_Add` (`self.Tests`) "Test_16_Copy_JSON" (and (== (`KismetMathLibrary.FTrunc` (`JsonFieldData.GetNumber` _returnvalue "copy")) 1) (`KismetStringLibrary.EqualEqual_StrStr` (`JsonFieldData.GetString` (`JsonFieldData.GetObject` _returnvalue "obj") "property") "value"))))

(fn `UserConstructionScript`)