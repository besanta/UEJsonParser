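; Avatar is a demo actor for JSON save serialization, with a tinted mesh and an HP/MaxHP text label.
; The construction script creates a dynamic material for its color, while Tick refreshes that color, the label and the stored Location.
; BeginPlay builds an Identity object with sample personal data and a capsule-derived size.
; Serialize writes the whole actor under the "Avatar" key; Unserialize is a stub returning false.
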(event `self.ReceiveBeginPlay`
  (bind _returnvalue (`|GenericCreateObject` "/Game/Blueprints/JsonDemoSaveGameFlag.JsonDemoSaveGameFlag_C" self "John" "Torino" 32 (* (`.SphereRadius` (`KismetSystemLibrary.GetComponentBounds` (`self.CapsuleComponent`))) 2.0) true))
  (set `self.Identity` _returnvalue))

(event `self.ReceiveTick`
  (params (DeltaSeconds :type "Float (single-precision)"))
  (`MaterialInstanceDynamic.SetVectorParameterValue` (`self.MID`) "Color" (`self.Color`))
  (`TextRenderComponent.K2_SetText` (`self.TextRender`) (`|FormatText` "{hp}/{mhp}" (`self.HP`) (`self.MaxHP`)))
  (set `self.Location` (`self.K2_GetActorLocation`)))

(fn `Serialize`
  (params (data :type "JsonFieldData Object Reference"))
  (returns (ReturnValue :type "JsonFieldData Object Reference"))
  (return (`JsonFieldData.SetUObject` data "Avatar" self)))

(fn `Unserialize`
  (params (data :type "JsonFieldData Object Reference"))
  (returns (ReturnValue :type Boolean))
  (return false))

(fn `UserConstructionScript`
  (bind _returnvalue (`PrimitiveComponent.CreateDynamicMaterialInstance` (`self.Mesh`) 0 "/Game/TutorialTPP_Mat.TutorialTPP_Mat" "None"))
  (bind _output_get (set `self.MID` _returnvalue))
  (`MaterialInstanceDynamic.SetVectorParameterValue` _output_get "Color" (`self.Color`)))