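; Ball actor that changes color according to how many times it has been hit by other Balls.
; The construction script creates a dynamic material instance on Sphere1 and applies the color for the current hit count.
; Each Sphere hit from another Ball increments the count and looks up a new color in the Ramp map, keeping the current one if no entry matches.
; Tick also pushes the current color to the material every frame.
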(event `self.ReceiveBeginPlay`)

(event `self.ReceiveTick`
  (params (DeltaSeconds :type "Float (single-precision)"))
  (`MaterialInstanceDynamic.SetVectorParameterValue` (`self.MID`) "Color" (`self.Color`)))

(event `DetermineColor`
  (bind (_value _returnvalue) (`BlueprintMapLibrary.Map_Find` (`self.Ramp`) (`self.Hits`)))
  (if _returnvalue
    (set `self.Color` _value)
    (`MaterialInstanceDynamic.SetVectorParameterValue` (`self.MID`) "Color" (`self.Color`))))

(event `self.Sphere.OnComponentHit`
  (params (HitComponent :type "PrimitiveComponent Object Reference") (OtherActor :type "Actor Object Reference") (OtherComp :type "PrimitiveComponent Object Reference") (NormalImpulse :type "Vector Structure") (Hit :type "HitResult Structure (by ref)"))
  (cast `/Game/Blueprints/Ball` OtherActor)
  (`/Engine/EditorBlueprintResources/StandardMacros.IncrementInt` (`self.Hits`)
    (:`  `
      (`self.DetermineColor`))))

(fn `UserConstructionScript`
  (bind _returnvalue (`PrimitiveComponent.CreateDynamicMaterialInstance` (`self.Sphere1`) 0 "/Game/TutorialTPP_Mat.TutorialTPP_Mat" "None"))
  (set `self.MID` _returnvalue)
  (`self.DetermineColor`))